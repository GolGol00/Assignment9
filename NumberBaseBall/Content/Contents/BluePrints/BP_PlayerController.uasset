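; Player controller for a networked chat system, linking the chat window widget to the BP_ChatMode game mode.
; After a short delay on BeginPlay, it finds Widget_ChatWindow and binds to its message dispatcher.
; Outgoing messages get the user ID prefixed and go to the game mode; received broadcasts print on screen, colored by server or client.
; Login events, including a client RPC variant, store the user ID and fire OnUserLogin.
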(event Custom|OnLoginWithID
  (params (UserId :type String))
  ;[1 1 1] UserID를 로그인했을떄 Host인지 Guest인지 판단해주는 함수
  (Default|CallOnUserLogin UserId)
  (Variables|Default|SetUserId UserId))

(event Custom|ClientRPC_ONLoginWithIn
  (params (userID :type String))
  ;[1 1 1] RPC를 클라이언트 전용으로 하나 만든다.
  (Default|CallOnUserLogin userID)
  (Variables|Default|SetUserId userID))

(event Custom|GotBroadcast
  (params (Msg :type String))
  ;[1 1 1] 메세지를 출력해주는 부분 여기를 클라이언트로해야 2번출력이안된다.
  (if (Networking|IsServer)
    (Development|PrintString Msg true true "(R=1.000000,G=0.000000,B=0.081139,A=1.000000)" 1e+01)
    (else
      (Development|PrintString Msg true true "(R=0.962442,G=1.000000,B=0.978911,A=1.000000)" 1e+01))))

(event Custom|OnsendMsgToServer
  (params (Msg :type Text))
  ;[1 1 1] 메세지를 서버나 다른 클라이언트에 넘겨주는 함수
  (bind _asbp_chat_mode (Utilities|Casting|CastToBP_ChatMode (Game|GetGameMode)))
  (Default|GotMessagefromClient _asbp_chat_mode (Utilities|String|Append (Variables|Default|GetUserId) " : " (Utilities|String|ToString(Text) Msg))))

(event EventBeginPlay
  ;[1 1 1] 모든 플레이어들에게 메세지 이벤트디스패쳐 독
  (if (not (Utilities|Enum|Equal(Enum) (Class|Actor|GetRemoteRole) "ROLE_None"))
    (Utilities|FlowControl|Delay 0.7)
    (bind _foundwidgets (Widget|GetAllWidgetsOfClass "/Game/Contents/Widgets/Widget_ChatWindow.Widget_ChatWindow_C" true))
    (bind _output_get (Variables|Default|SetWidget (Utilities|Array|Get(acopy) _foundwidgets)))
    (EventDispatchers|BindEventtoSetMessagetoUserController _output_get (EventDispatchers|CreateEvent :!event Custom|OnsendMsgToServer))))

(fn ConstructionScript)